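; BP_Collectibel is a weapon pickup actor that grants gameplay abilities when overlapped.
; Enable applies the configured skeletal or static weapon meshes, both in the construction script and on BeginPlay.
; On box overlap, any actor with an Ability System Component receives the configured ability, which is activated immediately.
; Successful activation also grants the sword equip and unequip abilities and gives the pickup a brief lifespan, destroying it.
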(event `self.ReceiveBeginPlay`
  ;[1 1 1] 预加载
  (`self.Enable`))

(event `Enable`
  (`|ExecutionSequence`
    (:`then_0`
      (`/Engine/EditorBlueprintResources/StandardMacros.IsValid` (`self.SetSkWeapon`)
        (:`Is Valid`
          (`SkeletalMeshComponent.SetSkeletalMeshAsset` (`self.SK_Weapon`) (`self.SetSkWeapon`)))))
    (:`then_1`
      (`/Engine/EditorBlueprintResources/StandardMacros.IsValid` (`self.SM_Weapon`)
        (:`Is Valid`
          (`StaticMeshComponent.SetStaticMesh` (`self.Weapon`) (`self.SM_Weapon`)))))))

(event `self.Box.OnComponentBeginOverlap`
  (params (OverlappedComponent :type "PrimitiveComponent Object Reference") (OtherActor :type "Actor Object Reference") (OtherComp :type "PrimitiveComponent Object Reference") (OtherBodyIndex :type Integer) (bFromSweep :type Boolean) (SweepResult :type "HitResult Structure (by ref)"))
  (bind _returnvalue (`AbilitySystemBlueprintLibrary.GetAbilitySystemComponent` OtherActor))
  (`/Engine/EditorBlueprintResources/StandardMacros.IsValid` _returnvalue
    (:`Is Valid`
      ;[1 1 1] 找到相应的技能
      (bind _returnvalue_2 (`AbilitySystemComponent.K2_GiveAbility` _returnvalue (`self.Ability Class`) 0 -1))
      ;[1 1 1] 激活相应的技能
      (bind _returnvalue_3 (`AbilitySystemComponent.TryActivateAbility` _returnvalue _returnvalue_2 true))
      (if _returnvalue_3
        (`self.SetLifeSpan` 0.1)
        (`AbilitySystemComponent.K2_GiveAbility` _returnvalue "/Game/00_Blueprints/00_Abilities/GA_EquipSword.GA_EquipSword_C" 0 -1)
        (`AbilitySystemComponent.K2_GiveAbility` _returnvalue "/Game/00_Blueprints/00_Abilities/GA_UnEquipSword.GA_UnEquipSword_C" 0 -1)))))

(fn `UserConstructionScript`
  ;[1 1 1] 构造脚本
  (`self.Enable`))